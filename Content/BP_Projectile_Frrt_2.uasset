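; BP_Projectile_Frrt_2 is a projectile that damages the player when its HitBox overlaps an actor tagged Player, then destroys itself.
; It ignores overlaps with actors tagged Bullet, Enemy or Drop.
; Any other overlapped actor has its display name printed before the projectile destroys itself without applying damage.
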(event `self.HitBox.OnComponentBeginOverlap`
  (params (OverlappedComponent :type "PrimitiveComponent Object Reference") (OtherActor :type "Actor Object Reference") (OtherComp :type "PrimitiveComponent Object Reference") (OtherBodyIndex :type Integer) (bFromSweep :type Boolean) (SweepResult :type "HitResult Structure (by ref)"))
  (if (`self.ActorHasTag` OtherActor "Player")
    (`GameplayStatics.ApplyDamage` OtherActor (`self.Damage`))
    (`self.K2_DestroyActor` :!label _label)
    (elif (not (or (`self.ActorHasTag` OtherActor "Bullet") (`self.ActorHasTag` OtherActor "Enemy") (`self.ActorHasTag` OtherActor "Drop")))
      (`KismetSystemLibrary.PrintString` (`KismetSystemLibrary.GetDisplayName` OtherActor))
      (goto _label))))

(fn `UserConstructionScript`)