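; Level 1 enemy that chases the player and deals contact damage.
; On BeginPlay it sets its health and runs AIMoveTo toward the player, then damages them and destroys itself when the move finishes.
; AnyDamage lowers and prints health; at zero it rarely spawns a health pickup, otherwise an EXP pickup carrying its drop amount.
; Only the EXP branch destroys the enemy.
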(event `self.ReceiveBeginPlay`
  (set `self.CurrentHealth` (`self.Health`))
  (bind _output_get (set `self.Player` (`GameplayStatics.GetPlayerCharacter` 0)))
  (`AITask_MoveTo.AIMoveTo` (`AIBlueprintHelperLibrary.GetAIController` self) (0.0 0.0 0.0) _output_get 10.0 "Enable" "Enable"
    (:`OnMoveFinished`
      (`GameplayStatics.ApplyDamage` _output_get 1.0)
      (`self.K2_DestroyActor`))))

(event `self.ReceiveAnyDamage`
  (params (Damage :type "Float (single-precision)") (DamageType :type "DamageType Object Reference") (InstigatedBy :type "Controller Object Reference") (DamageCauser :type "Actor Object Reference"))
  (bind _returnvalue (`self.GetTransform`))
  (bind _output_get (set `self.CurrentHealth` (- (`self.CurrentHealth`) Damage)))
  (`KismetSystemLibrary.PrintString` (`KismetStringLibrary.Conv_DoubleToString` _output_get))
  (if (<= _output_get 0.0)
    (if (<= (`KismetMathLibrary.RandomIntegerInRange` 1 100) 2)
      (`|SpawnActorFromClass` "/Game/ThirdPerson/Blueprints/BP_Health_Pickup.BP_Health_Pickup_C" _returnvalue "Undefined" "MultiplyWithRoot" null null)
      (else
        (bind _returnvalue_2 (`|SpawnActorFromClass` "/Game/ThirdPerson/Blueprints/BP_EXP_Pickup.BP_EXP_Pickup_C" _returnvalue "AdjustIfPossibleButAlwaysSpawn" "MultiplyWithRoot" null null))
        (set `/Game/ThirdPerson/Blueprints/BP_EXP_Pickup.ExpGain` (`self.EXPDropAmount`) _returnvalue_2)
        (`self.K2_DestroyActor`)))))

(fn `UserConstructionScript`)