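; Wave manager that spawns enemies around the player on a looping timer until wave 100 ends the game as a win.
; Each wave picks reachable points away from the player, rolls one of three enemy tiers by WaveLevel and scales health.
; Every fifth wave adjusts timer, count, health or level, adds score and resets the timer.
; The final wave destroys tagged enemies, saves the result to GameInstanceScore and opens EndScreen.
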(event `self.ReceiveBeginPlay`
  (`KismetSystemLibrary.K2_SetTimerDelegate` (delegate `CustomEvent`) (`self.WaveTimer`) true 0.0 1.0))

(event `CustomEvent`
  (bind _returnvalue (`self.K2_GetActorLocation` (`GameplayStatics.GetPlayerCharacter` 0)))
  (bind _returnvalue_2 (`KismetMathLibrary.MakeTransform` (`self.RandomLocation`)))
  (bind _randomlocation (`NavigationSystemV1.K2_GetRandomReachablePointInRadius` _returnvalue 1500.0 null null))
  (for _ (range 1 (+ (`self.EnemiesPerWave`) 1))
    (set `self.RandomLocation` _randomlocation)
    (while (< (`KismetMathLibrary.Vector_Distance` _returnvalue (`self.RandomLocation`)) 1000.0)
      (set `self.RandomLocation` _randomlocation))
    (`self.Determine Level`
      (:`LV1`
        (bind _returnvalue_3 (`|SpawnActorFromClass` "/Game/BP_Enemy_Frrt_Level_1.BP_Enemy_Frrt_Level_1_C" _returnvalue_2 "Undefined" "MultiplyWithRoot" null null))
        (set `/Game/BP_Enemy_Frrt_Level_1.Health` (* (`/Game/BP_Enemy_Frrt_Level_1.Health` _returnvalue_3) (`self.EnemyHPMult`)) _returnvalue_3))
      (:`LV2`
        (bind _returnvalue_4 (`|SpawnActorFromClass` "/Game/BP_Enemy_Frrt_Level_2.BP_Enemy_Frrt_Level_2_C" _returnvalue_2 "Undefined" "MultiplyWithRoot" null null))
        (set `/Game/BP_Enemy_Frrt_Level_2.Health` (* (`/Game/BP_Enemy_Frrt_Level_2.Health` _returnvalue_4) (`self.EnemyHPMult`)) _returnvalue_4))
      (:`LV3`
        (bind _returnvalue_5 (`|SpawnActorFromClass` "/Game/BP_Enemy_Frrt_Level_3.BP_Enemy_Frrt_Level_3_C" _returnvalue_2 "Undefined" "MultiplyWithRoot" null null))
        (set `/Game/BP_Enemy_Frrt_Level_3.Health` (* (`/Game/BP_Enemy_Frrt_Level_3.Health` _returnvalue_5) (`self.EnemyHPMult`)) _returnvalue_5))))
  (bind _result (`/Engine/EditorBlueprintResources/StandardMacros.IncrementInt` (`self.WaveNumber`))
    (:`  `
      (bind _returnvalue_6 (`KismetStringLibrary.Conv_IntToString` _result))
      (switch `string` _returnvalue_6
        (:`5`
          (set `self.WaveTimer` (- (`self.WaveTimer`) 0.1) :!label _label)
          (`KismetSystemLibrary.PrintString` (`KismetStringLibrary.Concat_StrStr` "Wave: " _returnvalue_6) :!label _label_2)
          (bind _asbp_third_person_character (cast `/Game/ThirdPerson/Blueprints/BP_ThirdPersonCharacter` (`GameplayStatics.GetPlayerCharacter` 0)))
          (set `/Game/ThirdPerson/Blueprints/BP_ThirdPersonCharacter.Score` (+ (`/Game/ThirdPerson/Blueprints/BP_ThirdPersonCharacter.Score` _asbp_third_person_character) (* (`self.WaveNumber`) (`self.WaveLevel`))) _asbp_third_person_character)
          (`KismetSystemLibrary.Delay` 0.0)
          (`KismetSystemLibrary.K2_SetTimerDelegate` (delegate `CustomEvent`) (`self.WaveTimer`) true))
        (:`10`
          (`/Engine/EditorBlueprintResources/StandardMacros.IncrementInt` (`self.EnemiesPerWave`) :!label _label_3
            (:`  `
              (goto _label_2))))
        (:`15`
          (goto _label))
        (:`20`
          (set `self.EnemyHPMult` (+ (`self.EnemyHPMult`) 0.5) :!label _label_4)
          (goto _label_2))
        (:`25`
          (goto _label_3))
        (:`30`
          (set `self.WaveTimer` (+ (`self.WaveTimer`) 0.4) :!label _label_5)
          (`/Engine/EditorBlueprintResources/StandardMacros.IncrementInt` (`self.WaveLevel`)
            (:`  `
              (goto _label_2))))
        (:`35`
          (goto _label_4))
        (:`40`
          (goto _label_3))
        (:`45`
          (goto _label))
        (:`50`
          (goto _label_4))
        (:`55`
          (set `self.EnemiesPerWave` (* (`self.EnemiesPerWave`) 2))
          (goto _label_2))
        (:`60`
          (goto _label))
        (:`65`
          (goto _label))
        (:`70`
          (goto _label_5))
        (:`75`
          (goto _label_3))
        (:`80`
          (goto _label_4))
        (:`85`
          (goto _label_3))
        (:`90`
          (goto _label))
        (:`95`
          (goto _label_3))
        (:`100`
          (bind _outactors (`GameplayStatics.GetAllActorsWithTag` "Enemy"))
          (for _array_element _outactors
            (`self.K2_DestroyActor` _array_element))
          (`KismetSystemLibrary.Delay` 0.2)
          (bind _asbp_third_person_character_2 (cast `/Game/ThirdPerson/Blueprints/BP_ThirdPersonCharacter` (`GameplayStatics.GetPlayerCharacter` 0)))
          (bind _output_get (set `/Game/ThirdPerson/Blueprints/BP_ThirdPersonCharacter.Winner` true _asbp_third_person_character_2))
          (bind _asgame_instance_score (cast `/Game/GameInstanceScore` (`GameplayStatics.GetGameInstance`)))
          (set `/Game/GameInstanceScore.Score` (`/Game/ThirdPerson/Blueprints/BP_ThirdPersonCharacter.Score` _asbp_third_person_character_2) _asgame_instance_score)
          (set `/Game/GameInstanceScore.Winner` _output_get _asgame_instance_score)
          (`GameplayStatics.OpenLevel` "EndScreen"))))))

(fn `UserConstructionScript`)