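; Level 2 Frrt enemy that wanders, constantly faces the player and shoots projectiles.
; Looping timers set at BeginPlay drive random navmesh moves within a small radius and spawn a projectile from its Sphere component along the actor's rotation.
; Tick turns it toward the player character.
; Damage lowers and prints its health; on death it drops either a rare health pickup or an EXP pickup carrying its drop amount, then destroys itself.
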(event `self.ReceiveBeginPlay`
  (`KismetSystemLibrary.K2_SetTimerDelegate` (delegate `MoveRandomly`) 2.0 true 0.0 2.5)
  (set `self.CurrentHealth` (`self.Health`))
  (set `self.Player` (`GameplayStatics.GetPlayerCharacter` 0))
  (`KismetSystemLibrary.K2_SetTimerDelegate` (delegate `Shoot`) 6.5 true))

(event `MoveRandomly`
  (`AITask_MoveTo.AIMoveTo` (`AIBlueprintHelperLibrary.GetAIController` self) (`NavigationSystemV1.K2_GetRandomReachablePointInRadius` (`self.K2_GetActorLocation`) 300.0 null null) null 1.0 "Enable" "Enable"))

(event `Shoot`
  (`|SpawnActorFromClass` "/Game/BP_Projectile_Frrt_2.BP_Projectile_Frrt_2_C" (`KismetMathLibrary.MakeTransform` (`SceneComponent.K2_GetComponentLocation` (`self.Sphere`)) (`self.K2_GetActorRotation`)) "Undefined" "MultiplyWithRoot" null null))

(event `self.ReceiveTick`
  (params (DeltaSeconds :type "Float (single-precision)"))
  (`self.K2_SetActorRotation` (`KismetMathLibrary.FindLookAtRotation` (`self.K2_GetActorLocation`) (`self.K2_GetActorLocation` (`GameplayStatics.GetPlayerCharacter` 0)))))

(event `self.ReceiveAnyDamage`
  (params (Damage :type "Float (single-precision)") (DamageType :type "DamageType Object Reference") (InstigatedBy :type "Controller Object Reference") (DamageCauser :type "Actor Object Reference"))
  (bind _returnvalue (`self.GetTransform`))
  (bind _output_get (set `self.CurrentHealth` (- (`self.CurrentHealth`) Damage)))
  (`KismetSystemLibrary.PrintString` (`KismetStringLibrary.Conv_DoubleToString` _output_get))
  (if (<= _output_get 0.0)
    (if (<= (`KismetMathLibrary.RandomIntegerInRange` 1 100) 5)
      (`|SpawnActorFromClass` "/Game/ThirdPerson/Blueprints/BP_Health_Pickup.BP_Health_Pickup_C" _returnvalue "Undefined" "MultiplyWithRoot" null null)
      (else
        (bind _returnvalue_2 (`|SpawnActorFromClass` "/Game/ThirdPerson/Blueprints/BP_EXP_Pickup.BP_EXP_Pickup_C" _returnvalue "AdjustIfPossibleButAlwaysSpawn" "MultiplyWithRoot" null null))
        (set `/Game/ThirdPerson/Blueprints/BP_EXP_Pickup.ExpGain` (`self.EXPDropAmount`) _returnvalue_2)))
    (`self.K2_DestroyActor`)))

(fn `UserConstructionScript`)